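; Bridge lock prop that a VR player opens by holding a key near it and twisting the hand.
; A looping timer polls gripped keys for proximity and controller roll, with mirrored angle limits per hand.
; Unlocking plays a sound and resets a countdown through a DoOnce.
; A second timer relocks it when time runs out, while Tick pushes state and remaining time to a clock widget.
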(event Custom|GetKey
  ;[1 1 1] Checks for key and player unlock interaction
  (bind _unlocked (Utilities|UnlockBridge)
    (:Out
      (if _unlocked
        (Utilities|FlowControl|DoOnce false :!label _label
          (:Completed
            (Audio|PlaySoundatLocation "/Game/HW2/Sounds/Lock.Lock" "0, 0, 0" "0, 0, 0" 1.0 1.0 0.0 0 0 0 0)
            (Variables|Default|SetUnlockTimeRemaining (Variables|Default|GetUnlockTime))
            (Rendering|SetVisibility (Variables|Default|GetPointLight) false false)))
        (else
          (goto _label Reset))))))

(event Custom|CountDownUnlock
  ;[1 1 1] If unlocked, counts down time and relocks when zero
  (if (Variables|Default|GetUnlocked)
    (bind _result (Math|Float|DecrementFloat (Variables|Default|GetUnlockTimeRemaining))
      (:%20%20
        (if (<= _result 0.0)
          (Variables|Default|SetUnlocked false)
          (Audio|PlaySoundatLocation "/Game/HW2/Sounds/LockRev.LockRev" "0, 0, 0" "0, 0, 0" 1.0 1.0 0.0 0 0 0 0)
          (Rendering|SetVisibility (Variables|Default|GetPointLight) false false))))))

(event EventBeginPlay
  (Rendering|SetVisibility (Variables|Default|GetPointLight) false false)
  (Utilities|Time|SetTimerbyFunctionName 0 "GetKey" 0.5 true)
  (Utilities|Time|SetTimerbyFunctionName 0 "CountDownUnlock" 1.0 true))

(event EventTick
  (params (DeltaSeconds :type Float%20%28single-precision%29))
  (bind _asbridge_clock (Utilities|Casting|CastToBridgeClock (UserInterface|GetUserWidgetObject (Variables|Default|GetClock))))
  (Variables|/Game/HW2/UI/BridgeClock.BridgeClock_C|SetBridgeState _asbridge_clock (Variables|Default|GetUnlocked))
  (Variables|/Game/HW2/UI/BridgeClock.BridgeClock_C|SetBridgeTime _asbridge_clock (Variables|Default|GetUnlockTimeRemaining)))

(fn ConstructionScript)