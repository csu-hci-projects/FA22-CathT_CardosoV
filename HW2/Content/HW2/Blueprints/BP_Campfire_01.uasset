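; Campfire actor that starts unlit, consumes nearby stick actors as fuel and warms the player while lit.
; Looping timers poll for wood, count down burn time, update the player and trigger a bonfire sound once per ignition.
; Added wood ignites the fire and extends burn time; as fuel runs low, light, flame particles and heat scale shrink until it goes out.
; Heat reaches C_HW2 as a proximity flag and scale.
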(event Custom|HeatPlayer
  ;[1 1 1] If player is nearby, set "Near Heat Source" variable.
  (bind _asc_hw2 (Utilities|Casting|CastToC_HW2 (Game|GetPlayerCharacter 0)))
  (Utilities|SendHeattoPlayer _asc_hw2 (and (< (Transformation|GetHorizontalDistanceTo _asc_hw2) 4e+02) (Variables|Default|GetIsLit)) (Variables|Default|GetHeatingScale)))

(event Custom|GetWood
  ;[1 1 1] Check for nearby wood. Consume wood and destroy wood actor.
  (bind _outactors (Actor|GetAllActorsOfClass "/Game/HW2/Blueprints/PB_Stick_01.PB_Stick_01_C"))
  (for _array_element _outactors
    (if (< (Transformation|GetHorizontalDistanceTo _array_element) 2e+01)
      (Utilities|AddWoodtoFire
        (:Out
          (Actor|DestroyActor _array_element))))))

(event Custom|BurnWood
  ;[1 1 1] Count down remaining burn time if lit.
  (if (Variables|Default|GetIsLit)
    (Variables|Default|SetBurnTimeRemaining (Math|Float|Max(Float) (- (Variables|Default|GetBurnTimeRemaining) 1.0) 0.0))
    (if (<= (Math|Float|Max(Float) (- (Variables|Default|GetBurnTimeRemaining) 1.0) 0.0) 3e+01)
      (Utilities|AdjustFlame (/ (Math|Float|Max(Float) (- (Variables|Default|GetBurnTimeRemaining) 1.0) 0.0) 3e+01)
        (:Out
          (if (Math|Float|NearlyEqual(Float) (Math|Float|Max(Float) (- (Variables|Default|GetBurnTimeRemaining) 1.0) 0.0) 0.0 1e-06)
            (Utilities|ExtinguishFire)))))))

(event Custom|PlaySound
  (if (Variables|Default|GetIsLit)
    (Utilities|FlowControl|DoOnce true :!label _label
      (:Completed
        (Audio|PlaySoundatLocation "/Game/HW2/Sounds/Bonfire.Bonfire" "0, 0, 0" "0, 0, 0" 2.0 1.0 0.0 0 0 0 0)))
    (else
      (goto _label Reset))))

(event EventBeginPlay
  (Utilities|ExtinguishFire
    (:Out
      (Utilities|Time|SetTimerbyFunctionName 0 "HeatPlayer" 0.5 true)
      (Utilities|Time|SetTimerbyFunctionName 0 "GetWood" 0.5 true)
      (Utilities|Time|SetTimerbyFunctionName 0 "BurnWood" 1.0 true)
      (Utilities|Time|SetTimerbyFunctionName 0 "PlaySound" 1.0 true))))

(fn ConstructionScript)