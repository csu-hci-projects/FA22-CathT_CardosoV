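; VR player pawn for a survival game with Heat and Cold stats shown on a HUD.
; Thumbsticks turn the pawn and move it by unswept root offsets, with sprint switching speed.
; Grab inputs line-trace from each motion controller to grip VRGripInterface components or actors, dropping on release.
; A looping timer updates the stats from exponential time-of-day curves around noon and midnight, adjusted near heat sources, then refreshes the HUD.
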(event Custom|UpdateStats
  ;[1 1 1] Update Heat/Cold based on time of day
  (bind (_heatout _coldout) (Utilities|UpdateStatsbyEnvironment)
    (:Out
      (bind (_heatout_2 _coldout_2) (Utilities|UpdateHUD _heatout _coldout)
        (:Out
          (Variables|Stats|SetHeat _heatout_2)
          (Variables|Stats|SetCold _coldout_2))))))

(event EventBeginPlay
  (Utilities|UpdateHUD 0.0 0.0
    (:Out
      (Utilities|Time|SetTimerbyFunctionName 0 "UpdateStats" 0.5 true))))

(event Collision|EventActorBeginOverlap
  (params (OtherActor :type Actor%20Object%20Reference)))

(event EventTick
  (params (DeltaSeconds :type Float%20%28single-precision%29)))

(event Input|ActionEvents|InputActionSprint
  (params (Key :type Key%20Structure))
  ;[1 1 1] Sprinting control
  (:Pressed
    (Utilities|StartSprinting))
  (:Released
    (Utilities|StopSprinting)))

(event Input|ActionEvents|InputActionGrabLeft
  (params (Key :type Key%20Structure))
  (bind _leftmotioncontroller (Variables|Default|GetLeftMotionController))
  (bind _returnvalue (Transformation|GetWorldLocation _leftmotioncontroller))
  ;[1 1 1] Object Grabbing
  (:Pressed
    (bind (_outhit _returnvalue_2) (Collision|LineTraceByChannel _returnvalue (+ _returnvalue (* (Math|Vector|GetForwardVector _leftmotioncontroller) (Variables|Selection|GetGrabDistance))) "TraceTypeQuery1" true 0 "None"))
    (if _returnvalue_2 ; If we hit something
      (CallFunction|AttemptGripfromTrace _outhit _leftmotioncontroller)))
  (:Released
    (bind _griparray (Class|GripMotionControllerComponent|GetAllGrips _leftmotioncontroller))
    (for _array_element _griparray
      (Class|GripMotionControllerComponent|DropObjectbyInterface _leftmotioncontroller 0 (.GripID (Utilities|Struct|BreakBPActorGripInformation _array_element)) "0, 0, 0" "0, 0, 0"))))

(event Input|ActionEvents|InputActionGrabRight
  (params (Key :type Key%20Structure))
  (bind _rightmotioncontroller (Variables|Default|GetRightMotionController))
  (bind _returnvalue (Transformation|GetWorldLocation _rightmotioncontroller))
  ;[1 1 1] Object Grabbing
  (:Pressed
    (bind (_outhit _returnvalue_2) (Collision|LineTraceByChannel _returnvalue (+ _returnvalue (* (Math|Vector|GetForwardVector _rightmotioncontroller) (Variables|Selection|GetGrabDistance))) "TraceTypeQuery1" true 0 "None"))
    (if _returnvalue_2 ; If we hit something
      (CallFunction|AttemptGripfromTrace _outhit _rightmotioncontroller)))
  (:Released
    (bind _griparray (Class|GripMotionControllerComponent|GetAllGrips _rightmotioncontroller))
    (for _array_element _griparray
      (Class|GripMotionControllerComponent|DropObjectbyInterface _rightmotioncontroller 0 (.GripID (Utilities|Struct|BreakBPActorGripInformation _array_element)) "0, 0, 0" "0, 0, 0"))))

(event Input|AxisEvents|InputAxisMovementAxisRight_X
  (params (AxisValue :type Float%20%28single-precision%29))
  ;[1 1 1] Turn camera with right thumbstick
  (Class|VRBaseCharacter|AddActorWorldRotationVR (Math|Rotator|MakeRotator 0.0 0.0 (* AxisValue (Variables|Movement|GetTurnRate))) true))

(event Input|AxisEvents|InputAxisMovementAxisLeft_X
  (params (AxisValue :type Float%20%28single-precision%29))
  ;[1 1 1] Thumbstick movement
  (Transformation|AddWorldOffset (Variables|Default|GetVRRootReference) (* (Math|Vector|ProjectVectorontoPlane (Math|Vector|GetRightVector (Variables|Default|GetVRRootReference)) "0.000000,0.000000,1.000000") (* AxisValue (Variables|Movement|GetMaxWalkSpeed))) false true))

(event Input|AxisEvents|InputAxisMovementAxisLeft_Y
  (params (AxisValue :type Float%20%28single-precision%29))
  ;[1 1 1] Thumbstick movement
  (Transformation|AddWorldOffset (Variables|Default|GetVRRootReference) (* (Math|Vector|ProjectVectorontoPlane (Math|Vector|GetForwardVector (Variables|Default|GetVRRootReference)) "0,0.000000,-1.000000") (* AxisValue (Variables|Movement|GetMaxWalkSpeed))) false true))

(fn ConstructionScript)

(fn ToggleMenu
  (params (bActiveMenuHandRight :type Boolean)))

(fn AttemptGripfromTrace
  (params (HitResult :type Hit%20Result%20Structure) (Hand%20Gripping :type Grip%20Motion%20Controller%20Component%20Object%20Reference))
  (bind (_bblockinghit _binitialoverlap _time _distance _location _impactpoint _normal _impactnormal _physmat _hitactor _hitcomponent) (Collision|BreakHitResult HitResult))
  (if (Utilities|DoesObjectImplementInterface _hitcomponent "/Script/VRExpansionPlugin.VRGripInterface") ; Check if the component implements our interface first
    ;[1 1 1] Grip an Component
    (bind _output_get (Variables|Default|SetSelected%20Component _hitcomponent))
    (bind _returnvalue (Class|VRGripInterface|DenyGripping(Message) _output_get 0)) ; Check if the grip interface is telling us that\nthis object doesn't want to be gripped.
    (if (not _returnvalue)
      (Class|GripMotionControllerComponent|GripObjectbyInterface Hand%20Gripping (Variables|Default|GetSelected%20Component) (Transformation|GetWorldTransform (Variables|Default|GetSelected%20Component)) false "None" "None" false) ; All good, the object wants to be gripped.\nLets grip by interface and pass in the world transform\nthat we want to use.
    )
    (elif (Utilities|DoesObjectImplementInterface _hitactor "/Script/VRExpansionPlugin.VRGripInterface") ; If not then check the actor
      ;[1 1 1] Grip an Actor
      (bind _output_get_2 (Variables|Selection|SetSelected%20Actor _hitactor))
      (bind _returnvalue_2 (Class|VRGripInterface|DenyGripping(Message) _output_get_2 0))
      (if (not _returnvalue_2)
        (Class|GripMotionControllerComponent|GripObjectbyInterface Hand%20Gripping (Variables|Selection|GetSelected%20Actor) (Transformation|GetActorTransform (Variables|Selection|GetSelected%20Actor)) false "None" "None" false)))))

(fn StatStepbyTime
  (bind _timeofday (Variables|Stats|GetTimeOfDay))
  (bind _acceleratorfactor (Variables|Stats|GetAcceleratorFactor))
  (bind _acceleratorscale (Variables|Stats|GetAcceleratorScale))
  (bind _returnvalue (- 0.0 _timeofday))
  (bind _returnvalue_2 (- 12.0 _timeofday))
  (bind _returnvalue_3 (- 24.0 _timeofday))
  (bind _returnvalue_4 (Math|Float|Absolute(Float) _returnvalue_2))
  (bind _returnvalue_5 (Math|Float|Absolute(Float) _returnvalue_3))
  (bind _returnvalue_6 (Math|Float|Absolute(Float) _returnvalue))
  (bind _returnvalue_7 (* _returnvalue_6 _acceleratorfactor))
  (bind _returnvalue_8 (* _returnvalue_4 _acceleratorfactor))
  (bind _returnvalue_9 (* _returnvalue_5 _acceleratorfactor))
  (bind _returnvalue_10 (Class|KismetMathLibrary|Exp _returnvalue_8))
  (bind _returnvalue_11 (Class|KismetMathLibrary|Exp _returnvalue_9))
  (bind _returnvalue_12 (Class|KismetMathLibrary|Exp _returnvalue_7))
  (bind _returnvalue_13 (/ 1.0 _returnvalue_12))
  (bind _returnvalue_14 (/ 1.0 _returnvalue_10))
  (bind _returnvalue_15 (/ 1.0 _returnvalue_11))
  (bind _returnvalue_16 (* _returnvalue_14 _acceleratorscale))
  (bind _returnvalue_17 (* _returnvalue_13 _acceleratorscale))
  (bind _returnvalue_18 (* _returnvalue_15 _acceleratorscale))
  (if (Math|Float|InRange(Float) _timeofday 6.0 18.0 true false)
    (bind _result (Math|Float|NegateFloat _returnvalue_16)
      (:%20%20
        (return _returnvalue_16 _result)))
    (elif (Math|Float|InRange(Float) _timeofday 18.0 24.0 true false)
      (bind _result_2 (Math|Float|NegateFloat _returnvalue_18)
        (:%20%20
          (return _result_2 _returnvalue_18)))
      (else
        (bind _result_3 (Math|Float|NegateFloat _returnvalue_17)
          (:%20%20
            (return _result_3 _returnvalue_17)))))))

(fn StatStepbyHeatSource
  (params (EnvHeatStep :type Float%20%28double-precision%29) (EnvColdStep :type Float%20%28double-precision%29))
  (bind _returnvalue (Math|Float|Absolute(Float) EnvColdStep))
  (bind _heatsourcescale (Variables|Heating|GetHeatSourceScale))
  (bind _heatsourcecoldstep (Variables|Heating|GetHeatSourceColdStep))
  (bind _returnvalue_2 (* _heatsourcescale _heatsourcecoldstep))
  (bind _returnvalue_3 (+ _returnvalue_2 _returnvalue))
  (bind _returnvalue_4 (* _returnvalue_3 -1.0))
  (if (Variables|Heating|GetNearHeatSource)
    (if (< EnvHeatStep 0.0)
      (return (/ (Math|Float|Absolute(Float) EnvHeatStep) 2.0) _returnvalue_4)
      (else
        (return (* (Variables|Heating|GetHeatSourceHeatStep) _heatsourcescale) _returnvalue_4)))
    (else
      (return 0.0 0.0))))