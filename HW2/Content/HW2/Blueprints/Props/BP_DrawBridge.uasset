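; BP_DrawBridge is a drawbridge prop that raises or lowers according to its Lifting flag, which is not set within this file.
; A looping timer started at BeginPlay calls MoveBridge, stepping local roll in fixed increments between 0 and 72 degrees instead of using Tick.
; After each step, PlaySound triggers the drawbridge sound at world origin once while mid-range, re-arming when the roll reaches either limit.
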(event Custom|MoveBridge
  (bind _defaultsceneroot (Variables|Default|GetDefaultSceneRoot))
  (bind _lifting (Variables|Default|GetLifting))
  (bind _returnvalue (Transformation|GetSocketRotation _defaultsceneroot "None"))
  (if (and (< (.roll _returnvalue) 72.0) _lifting)
    (Transformation|AddActorLocalRotation (Math|Rotator|MakeRotator 0.125 0.0 0.0) false false)
    (Utilities|PlaySound (.roll _returnvalue) :!label _label)
    (elif (and (not _lifting) (> (.roll _returnvalue) 0.0))
      (Transformation|AddActorLocalRotation (Math|Rotator|MakeRotator -0.125 0.0 0.0) false false)
      (goto _label))))

(event EventBeginPlay
  (Utilities|Time|SetTimerbyFunctionName 0 "MoveBridge" 0.01 true))

(event Collision|EventActorBeginOverlap
  (params (OtherActor :type Actor%20Object%20Reference)))

(event EventTick
  (params (DeltaSeconds :type Float%20%28single-precision%29)))

(fn ConstructionScript)